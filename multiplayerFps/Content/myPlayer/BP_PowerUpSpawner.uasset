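; Power-up spawner actor that places a BP_MasterPowerUp at a random point inside its Box component.
; BeginPlay and a bound respawn event both call SRV_SpawnPowerUp, which waits a short random delay, spawns the actor and stores it in PowerUp.
; PowerUp's OnRep requests another spawn when the reference is invalid and prints debug strings in both branches.
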(event Custom|SRV_SpawnPowerUp
  (bind _box (Variables|Default|GetBox))
  (Utilities|FlowControl|Delay (Math|Random|RandomFloatinRange 1.0 2.0))
  (bind _returnvalue (Game|SpawnActorfromClass "/Game/myPlayer/BP_MasterPowerUp.BP_MasterPowerUp_C" (Math|Transform|MakeTransform (Math|Random|RandomPointinBoundingBox (Transformation|GetWorldLocation _box) (Components|Box|GetScaledBoxExtent _box)) "0, 0, 0" "1,1,1") "AlwaysSpawn" self 0))
  (Variables|Default|SetPowerUp _returnvalue))

(event Custom|RespawnPowerUp_Event
  (CallFunction|SRVSpawnPowerUp))

(event EventBeginPlay
  (CallFunction|SRVSpawnPowerUp)
  (EventDispatchers|BindEventtoRespawnPowerUp (delegate Custom|RespawnPowerUp_Event)))

(fn ConstructionScript)

(fn OnRepPowerUp
  (Utilities|IsValid (Variables|Default|GetPowerUp)
    (:Is%20Valid
      (Development|PrintString "1"))
    (:Is%20Not%20Valid
      (CallFunction|SRVSpawnPowerUp)
      (Development|PrintString "2"))))