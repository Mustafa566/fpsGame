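; BP_MasterPowerUp is a power-up pickup that is collected when a spear overlaps its cube.
; The overlap runs a hit event, named as a server call, that continues only for a spear hitting a power-up owned by a BP_PowerUpSpawner.
; It asks the spawner to respawn, sends the spear's player owner to the first BP_RocketSpear in the world for a power-up message, then destroys itself.
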(event OnComponentBeginOverlap(Cube)
  (params (OverlappedComponent :type Primitive%20Component%20Object%20Reference) (OtherActor :type Actor%20Object%20Reference) (OtherComp :type Primitive%20Component%20Object%20Reference) (OtherBodyIndex :type Integer) (bFromSweep :type Boolean) (SweepResult :type Hit%20Result%20Structure%20%28by%20ref%29))
  (CallFunction|SRVonHit OtherActor))

(event Custom|SRV_OnHit
  (params (OtherActor :type Actor%20Object%20Reference))
  (bind _asspear (Utilities|Casting|CastTospear OtherActor))
  (bind _asbp_power_up_spawner (Utilities|Casting|CastToBP_PowerUpSpawner (Components|GetOwner)))
  (Default|CallRespawnPowerUp _asbp_power_up_spawner)
  (bind _outactors (Actor|GetAllActorsOfClass "/Game/myPlayer/spear/BP_RocketSpear.BP_RocketSpear_C"))
  (Class|PowerUpInterface|ActivatePowerUp(Message) (Utilities|Array|Get(acopy) _outactors) (Variables|/Game/myPlayer/spear/spear.spear_C|GetplayerOwner _asspear))
  (Actor|DestroyActor))

(fn ConstructionScript)