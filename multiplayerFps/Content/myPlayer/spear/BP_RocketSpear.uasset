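; Rocket spear power-up that, on activation, spawns a volley of child spears tied to the opposing player.
; ActivatePowerUp searches all player actors and picks the first that is not the activating player as the enemy.
; On the authority only, a loop spawns scaled-down Spear_Child actors at the power-up's location, passing that enemy as their PlayerOwner.
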(event EventBeginPlay
  (|CallParentFunction) ; This node is disabled and will not be called.\nDrag off pins to build functionality.
)

(event Collision|EventActorBeginOverlap
  (params (OtherActor :type Actor%20Object%20Reference))
  (|CallParentFunction OtherActor) ; This node is disabled and will not be called.\nDrag off pins to build functionality.
)

(event EventTick
  (params (DeltaSeconds :type Float%20%28single-precision%29))
  (|CallParentFunction DeltaSeconds) ; This node is disabled and will not be called.\nDrag off pins to build functionality.
)

(event EventActivatePowerUp
  (params (MyPlayer :type My%20Player%20Object%20Reference))
  (bind _outactors (Actor|GetAllActorsOfClass "/Game/myPlayer/myPlayer.myPlayer_C"))
  (bind _array_element (Utilities|Array|ForEachLoopwithBreak _outactors :!label _label)
    (:LoopBody
      (if (!= _array_element MyPlayer)
        (Variables|Default|SetEnemyPlayer _array_element)
        (goto _label Break)))
    (:Completed
      (Networking|SwitchHasAuthority
        (:Authority
          (for _index (range 0 5)
            (Game|SpawnActorfromClass "/Game/myPlayer/spear/spear_Child.spear_Child_C" (Math|Transform|MakeTransform (Transformation|GetActorLocation) "0, 0, 0" "0.200000,0.200000,0.200000") "AdjustIfPossibleButAlwaysSpawn" 0 (Variables|Default|GetEnemyPlayer) 0)))))))

(fn ConstructionScript
  (|CallParentFunction))